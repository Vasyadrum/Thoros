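; BP_BaseInventoryItem is the base world pickup actor for a grid inventory.
; On BeginPlay it builds a BP_BaseItemObject when none is set, passing its grid size, icon, rotation setting and own class.
; Interact offers that object to the given InventoryComponent through TryAddItem and, on success, calls ServerDestroyItem to remove the actor.
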(event `self.ReceiveBeginPlay`
  (if (not (`KismetSystemLibrary.IsValid` (`self.ItemObject`)))
    (bind _itemobject (`self.GetDefaultItemObject`))
    (set `self.ItemObject` _itemobject)))

(event `/Game/Thoros/Inventory/BPI_Interact.Interact`
  (params (InventoryComponent :type "/Game/Thoros/Inventory/BPC_Inventory Object Reference"))
  (bind _added (`/Game/Thoros/Inventory/BPC_Inventory.TryAddItem` InventoryComponent (`self.ItemObject`)))
  (if _added
    (`self.ServerDestroyItem`)))

(event `ServerDestroyItem`
  (`self.K2_DestroyActor`))

(fn `GetDefaultItemObject`
  (returns (ItemObject :type "/Game/Thoros/Inventory/BP_BaseItemObject Object Reference"))
  (bind (_item_size_x _item_size_y) (`KismetMathLibrary.BreakVector2D` (`self.Item Size`)))
  (bind _returnvalue (`|GenericCreateObject` self "/Game/Thoros/Inventory/BP_BaseItemObject.BP_BaseItemObject_C" (make `IntPoint` (`KismetMathLibrary.FTrunc` _item_size_x) (`KismetMathLibrary.FTrunc` _item_size_y)) (`self.Icon`) (`self.Item Rotate`) (`GameplayStatics.GetObjectClass` self)))
  (return _returnvalue))

(fn `UserConstructionScript`)